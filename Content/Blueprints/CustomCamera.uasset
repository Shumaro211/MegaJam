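; CustomCamera is a player camera manager that drives the view from the top-down character's camera and confines it to fixed bounds.
; On BeginPlay it caches the Camera of BP_TopDownCharacter.
; BlueprintUpdateCamera copies that camera's transform with a fixed FOV, clamping X and Y when the Player variable is true or passing location through otherwise.
; The upper Y limit scales with camera height.
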(event EventBeginPlay
  (bind _asbp_top_down_character (Utilities|Casting|CastToBP_TopDownCharacter (Game|Player|GetPlayerPawn 0)))
  (Variables|Default|SetCamera (Variables|/Game/TopDown/Blueprints/BP_TopDownCharacter.BP_TopDownCharacter_C|GetCamera _asbp_top_down_character)))

(event Collision|EventActorBeginOverlap
  (params (OtherActor :type Actor%20Object%20Reference)))

(event EventTick
  (params (DeltaSeconds :type Float%20%28single-precision%29)))

(fn ConstructionScript)

(fn BlueprintUpdateCamera
  (params (CameraTarget :type Actor%20Object%20Reference))
  (bind _camera (Variables|Default|GetCamera))
  (bind _camera_2 (Variables|Default|GetCamera))
  (bind _returnvalue (Transformation|GetWorldTransform _camera))
  (bind _returnvalue_2 (Transformation|GetWorldTransform _camera_2))
  (if (Variables|Default|GetPlayer?)
    (return (Math|Vector|MakeVector (Math|Float|Clamp(Float) (.x (.location _returnvalue_2)) 1703.029961 2842.012735) (Math|Float|Clamp(Float) (.y (.location _returnvalue_2)) -1.1e+03 (+ (/ (.z (.location _returnvalue_2)) 4e+01) 1.1e+03)) (.z (.location _returnvalue_2))) (.rotation _returnvalue_2) 55.0 true)
    (else
      (return (.location _returnvalue) (.rotation _returnvalue) 55.0 true))))