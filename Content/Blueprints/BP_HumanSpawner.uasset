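; BP_HumanSpawner is an actor that spawns a few BP_Human characters at random spots when play begins.
; It reads the game count from BP_GameInstance and spawns one extra human if any games are already recorded.
; Each spawn picks from the Points array in local space, gives the human its default controller, then removes a separately re-rolled random point, so positions can repeat.
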(event EventBeginPlay
  (bind _points (Variables|Default|GetPoints))
  (bind (_outitem _outindex) (Utilities|Array|Random _points))
  (bind _asbp_game_instance (Utilities|Casting|CastToBP_GameInstance (Game|GetGameInstance)))
  (for _index (range 1 (Math|Integer|SelectInt 3 2 (> (Variables|/Game/Blueprints/BP_GameInstance.BP_GameInstance_C|GetGames _asbp_game_instance) 0)))
    (bind _returnvalue (Game|SpawnActorfromClass "/Game/ThirdPerson/Blueprints/BP_Human.BP_Human_C" (Math|Conversions|ToTransform(Vector) (Math|Transform|TransformLocation (Transformation|GetActorTransform) _outitem)) "AdjustIfPossibleButAlwaysSpawn" "MultiplyWithRoot" 0 0))
    (Pawn|SpawnDefaultController _returnvalue)
    (Utilities|Array|RemoveIndex _points _outindex)))

(fn ConstructionScript)