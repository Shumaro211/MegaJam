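; BP_Grid is a grid cell actor that is Empty, Fill or Walkable, with Special and Movable options.
; The construction script removes the cube and darkens the spotlight for Empty and Walkable, keeps the cube for Fill, and swaps its material when Movable.
; On BeginPlay, Fill cells set the nav modifier's area class and make the cube block pawn and world channels.
; A BP_Minion entering the box turns the spotlight on.
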(event OnComponentBeginOverlap(Box)
  (params (OverlappedComponent :type Primitive%20Component%20Object%20Reference) (OtherActor :type Actor%20Object%20Reference) (OtherComp :type Primitive%20Component%20Object%20Reference) (OtherBodyIndex :type Integer) (bFromSweep :type Boolean) (SweepResult :type Hit%20Result%20Structure%20%28by%20ref%29))
  (Utilities|Casting|CastToBP_Minion OtherActor)
  (Rendering|Components|Light|SetIntensity (Variables|Default|GetSpotLight) 5e+03))

(event EventBeginPlay
  (bind _cube (Variables|Default|GetCube))
  (switch Utilities|FlowControl|Switch|SwitchonStates (Variables|Default|GetState)
    (:NewEnumerator1
      (Class|NavModifierComponent|SetAreaClass (Variables|Default|GetNavModifier))
      (Collision|SetCollisionResponsetoChannel _cube "ECC_Pawn" "ECR_Block")
      (Collision|SetCollisionResponsetoChannel _cube "ECC_WorldStatic" "ECR_Block")
      (Collision|SetCollisionResponsetoChannel _cube "ECC_WorldDynamic" "ECR_Block"))))

(event Collision|EventActorBeginOverlap
  (params (OtherActor :type Actor%20Object%20Reference)))

(event EventTick
  (params (DeltaSeconds :type Float%20%28single-precision%29)))

(fn ConstructionScript
  (Utilities|FlowControl|Sequence
    (:then_0
      (switch Utilities|FlowControl|Switch|SwitchonStates (Variables|Default|GetState)
        (:NewEnumerator0
          (Rendering|Components|Light|SetIntensity (Variables|Default|GetSpotLight) 0.0 :!label _label)
          (Components|DestroyComponent (Variables|Default|GetCube))
          (Rendering|SetVisibility (Variables|Default|GetCube) false false))
        (:NewEnumerator1
          (Rendering|SetVisibility (Variables|Default|GetCube) true false)
          (if (not (Variables|Default|GetSpecial?))
            (Rendering|Components|Light|SetIntensity (Variables|Default|GetSpotLight) 0.0)))
        (:NewEnumerator3
          (goto _label))))
    (:then_1
      (if (Variables|Default|GetMovable)
        (Rendering|Material|SetMaterial (Variables|Default|GetCube) 0 "/Game/Blueprints/old/NewMaterial.NewMaterial")))))