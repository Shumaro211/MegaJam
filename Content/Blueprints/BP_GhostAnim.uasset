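; Ghost scare actor that animates a guest running along a spline alongside a screaming ghost lady.
; Called swaps one skeletal mesh component to one of three guest models by Selection, loops its run animation, and plays the Susto timeline to move it along the spline with a yaw correction.
; After a short delay it resets the GhostLady_Scream anim instance's transition; a separate Tension event plays a 2D tension sound.
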(event Custom|Called
  (params (Selection :type Integer))
  (bind _spline (Variables|Default|GetSpline))
  (bind _guestbigguy_animated (Variables|Default|GetGuestBigGuy_animated))
  (bind _guestbigguy_animated_2 (Variables|Default|GetGuestBigGuy_animated))
  (Utilities|FlowControl|Sequence
    (:then_0
      (switch int Selection
        (:0
          (Components|SkeletalMesh|SetSkeletalMeshAsset _guestbigguy_animated "/Game/Art/Characters/GuestShortGuy/GuestShortGuy_animated.GuestShortGuy_animated")
          (Components|Animation|SetAnimation _guestbigguy_animated_2 "/Game/Art/Characters/GuestShortGuy/GuestShortGuy_animated_Run.GuestShortGuy_animated_Run")
          (Components|Animation|PlayAnimation _guestbigguy_animated_2 "/Game/Art/Characters/GuestShortGuy/GuestShortGuy_animated_Run.GuestShortGuy_animated_Run" true)
          (bind _newtrack_0 (Timeline|Susto PlayFromStart)
            (:Update
              (Transformation|SetRelativeTransform (Variables|Default|GetGuestBigGuy_animated) (Math|Transform|MakeTransform (.location (Spline|GetTransformatDistanceAlongSpline _spline (Math|Float|Lerp 0.0 (Spline|GetDistanceAlongSplineatSplinePoint _spline 4) _newtrack_0) "Local" false)) (Math|Rotator|MakeRotator (.roll (.rotation (Spline|GetTransformatDistanceAlongSpline _spline (Math|Float|Lerp 0.0 (Spline|GetDistanceAlongSplineatSplinePoint _spline 4) _newtrack_0) "Local" false))) (.pitch (.rotation (Spline|GetTransformatDistanceAlongSpline _spline (Math|Float|Lerp 0.0 (Spline|GetDistanceAlongSplineatSplinePoint _spline 4) _newtrack_0) "Local" false))) (+ (.yaw (.rotation (Spline|GetTransformatDistanceAlongSpline _spline (Math|Float|Lerp 0.0 (Spline|GetDistanceAlongSplineatSplinePoint _spline 4) _newtrack_0) "Local" false))) -9e+01)) "1.000000,1.000000,1.000000") false false))))
        (:1
          (Components|SkeletalMesh|SetSkeletalMeshAsset _guestbigguy_animated "/Game/Art/Characters/GuestGirl/GuestGirl_animated.GuestGirl_animated")
          (Components|Animation|SetAnimation _guestbigguy_animated "/Game/Art/Characters/GuestGirl/GuestGirl_animated_Run.GuestGirl_animated_Run")
          (Components|Animation|PlayAnimation _guestbigguy_animated_2 "/Game/Art/Characters/GuestGirl/GuestGirl_animated_Run.GuestGirl_animated_Run" true)
          (Timeline|Susto PlayFromStart))
        (:2
          (Components|SkeletalMesh|SetSkeletalMeshAsset _guestbigguy_animated_2 "/Game/Art/Characters/GuestBigGuy/GuestBigGuy_animated.GuestBigGuy_animated")
          (Components|Animation|SetAnimation _guestbigguy_animated_2 "/Game/Art/Characters/GuestBigGuy/GuestBigGuy_animated_Run.GuestBigGuy_animated_Run")
          (Components|Animation|PlayAnimation _guestbigguy_animated_2 "/Game/Art/Characters/GuestBigGuy/GuestBigGuy_animated_Run.GuestBigGuy_animated_Run" true)
          (Timeline|Susto PlayFromStart))))
    (:then_1
      (Utilities|FlowControl|Delay 0.3)
      (bind _asghost_lady_scream (Utilities|Casting|CastToGhostLady_Scream (Components|SkeletalMesh|GetAnimInstance (Variables|Default|GetSkeletalMesh))))
      (Default|ResetTransition _asghost_lady_scream))))

(event Custom|Tension
  (Audio|PlaySound2D "/Game/Art/Audio/PM_SFX_Ghost_Tension_01.PM_SFX_Ghost_Tension_01" 1.0 1.0 0.0 0 0))

(fn ConstructionScript)