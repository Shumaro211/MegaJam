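; Behavior tree task that sends a human AI to investigate an interactable stored in the blackboard.
; It moves the pawn to a random reachable point near the interactable's Look component.
; The human's Fear is mapped to extra acceptance radius, so more frightened humans can stop farther away.
; The task reports success whether the move succeeds or fails; a RandomPatrol call is left unconnected.
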(event EventReceiveExecuteAI
  (params (OwnerController :type AI%20Controller%20Object%20Reference) (ControlledPawn :type Pawn%20Object%20Reference))
  (bind _asbp_human (Utilities|Casting|CastToBP_Human ControlledPawn))
  (bind _asbp_interactable_master (Utilities|Casting|CastToBP_InteractableMaster (AI|BehaviorTree|GetBlackboardValueasActor (Variables|Default|Getblackboard))))
  (AI|AIMoveTo ControlledPawn (.RandomLocation (AI|Navigation|GetRandomReachablePointinRadius (Transformation|GetWorldLocation (Variables|/Game/Blueprints/Interacts/BP_InteractableMaster.BP_InteractableMaster_C|GetLook _asbp_interactable_master)) 3e+01 0 0)) 0 (+ (Variables|Default|GetAcceptance%20Radius) (Math|Float|MapRangeClamped (Math|Conversions|ToFloat(Integer) (Variables|/Game/ThirdPerson/Blueprints/BP_Human.BP_Human_C|GetFear _asbp_human)) 0.0 1e+02 0.0 1.4e+02)) true
    (:OnSuccess
      (AI|BehaviorTree|FinishExecute true))
    (:OnFail
      (AI|BehaviorTree|FinishExecute true))))