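; Behavior tree task that walks a BP_Human pawn to the BP_InteractableMaster actor stored in the blackboard.
; BP_Moving targets are followed as actors with a widened acceptance radius; others use a random reachable point near their Look component.
; Success finishes the task, but failure is reported only on the random-point branch, and failed casts never finish it.
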(event EventReceiveExecuteAI
  (params (OwnerController :type AI%20Controller%20Object%20Reference) (ControlledPawn :type Pawn%20Object%20Reference))
  (bind _acceptance_radius (Variables|Default|GetAcceptance%20Radius))
  (Utilities|Casting|CastToBP_Human ControlledPawn)
  (bind _asbp_interactable_master (Utilities|Casting|CastToBP_InteractableMaster (AI|BehaviorTree|GetBlackboardValueasActor (Variables|Default|Getblackboard))))
  (bind _asbp_moving (Utilities|Casting|CastToBP_Moving _asbp_interactable_master)
    (:then
      (AI|AIMoveTo ControlledPawn "0, 0, 0" _asbp_moving (+ _acceptance_radius 34.0) false
        (:OnSuccess
          (AI|BehaviorTree|FinishExecute true :!label _label))))
    (:CastFailed
      (AI|AIMoveTo ControlledPawn (.RandomLocation (AI|Navigation|GetRandomReachablePointinRadius (Transformation|GetWorldLocation (Variables|/Game/Blueprints/Interacts/BP_InteractableMaster.BP_InteractableMaster_C|GetLook _asbp_interactable_master)) 3e+01 0 0)) 0 _acceptance_radius false
        (:OnSuccess
          (goto _label))
        (:OnFail
          (AI|BehaviorTree|FinishExecute false))))))