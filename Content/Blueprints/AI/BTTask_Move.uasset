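; Behavior tree task that walks an AI_NPC along spline patrol paths, one point per execution.
; On execute it takes the closest patrol if none is set, or randomly switches after several points, then picks the current and next spline points.
; Each tick slides a target actor along the spline at constant speed while AIMoveTo chases it.
; Arrival near the next point finishes the task, sometimes after a random pause.
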(event EventReceiveExecuteAI
  (params (OwnerController :type AI%20Controller%20Object%20Reference) (ControlledPawn :type Pawn%20Object%20Reference))
  (bind _asai_npc (Utilities|Casting|CastToAI_NPC OwnerController))
  (Variables|Default|SetController _asai_npc)
  (Utilities|FlowControl|Sequence
    (:then_0
      (Utilities|IsValid (Variables|/Game/ThirdPerson/Blueprints/AI/AI_NPC.AI_NPC_C|GetCurrentActor (Variables|Default|GetController))
        (:Is%20Valid
          (if (> (Variables|Default|GetPointsNumber) 3)
            (if (> (Variables|Default|GetPointsNumber) 5)
              (Variables|Default|SetPointsNumber 0 :!label _label)
              (Default|RandomPatrol (Variables|Default|GetController))
              (elif (Math|Random|RandomBool)
                (goto _label)
                (else
                  _)))))
        (:Is%20Not%20Valid
          (Default|ClosestPatrol (Variables|Default|GetController))))
      (bind _point_index (Default|Path-FindClosestPathPoint (Variables|Default|GetController) ControlledPawn false (Variables|/Game/ThirdPerson/Blueprints/AI/AI_NPC.AI_NPC_C|GetCurrentActor (Variables|Default|GetController))))
      (Variables|Default|SetCurrent%20Point _point_index))
    (:then_1
      (if (== (Variables|Default|GetCurrent%20Point) (Variables|Default|GetNext%20Point))
        (if (> (+ (Variables|Default|GetCurrent%20Point) 1) (- (Spline|GetNumberOfSplinePoints (Variables|/Game/ThirdPerson/Blueprints/AI/BT_PatrolPoint.BT_PatrolPoint_C|GetSpline (Variables|/Game/ThirdPerson/Blueprints/AI/AI_NPC.AI_NPC_C|GetCurrentActor (Variables|Default|GetController)))) 1))
          (Variables|Default|SetNext%20Point 0)
          (else
            (Variables|Default|SetNext%20Point (+ (Variables|Default|GetCurrent%20Point) 1))))
        (else
          (Variables|Default|SetNext%20Point (Variables|Default|GetCurrent%20Point)))))
    (:then_2
      ;[1 1 1] Step 3) Save Spline Component To Variable
      (Variables|Default|SetTrack (Variables|/Game/ThirdPerson/Blueprints/AI/BT_PatrolPoint.BT_PatrolPoint_C|GetSpline (Variables|/Game/ThirdPerson/Blueprints/AI/AI_NPC.AI_NPC_C|GetCurrentActor (Variables|Default|GetController))))
      (Variables|Default|SetTarget%20Point%20to%20Follow (Variables|/Game/ThirdPerson/Blueprints/AI/AI_NPC.AI_NPC_C|GetTarget%20Point%20To%20Follow (Variables|Default|GetController))))
    (:then_3
      ;[1 1 1] Save Distances To Variables
      (Variables|Default|SetCurrent%20Distance (Spline|GetDistanceAlongSplineatSplinePoint (Variables|Default|GetTrack) (Variables|Default|GetCurrent%20Point)))
      (Variables|Default|SetNext%20Distance (Spline|GetDistanceAlongSplineatSplinePoint (Variables|Default|GetTrack) (Variables|Default|GetNext%20Point))))
    (:then_4
      ;[0.5083 1 0.2972] Step 3) Move AI and when Current Distance Nearly Equal Target Spine Point Distance Finish Execute
      (Utilities|FlowControl|DoOnce false) ; enters at Reset
    )))

(event EventReceiveTickAI
  (params (OwnerController :type AI%20Controller%20Object%20Reference) (ControlledPawn :type Pawn%20Object%20Reference) (DeltaSeconds :type Float%20%28single-precision%29))
  (bind _track (Variables|Default|GetTrack))
  (bind _target_point_to_follow (Variables|Default|GetTarget%20Point%20to%20Follow))
  (Variables|Default|SetDelta%20Seconds DeltaSeconds)
  (Utilities|FlowControl|Sequence
    (:then_0
      ;[0.4122 0.5417 0.109] Step 1) Interpolate Current Distance To Next Path Point
      ;;[0.3485 0.6719 0.2556] Interpolation Constant (Linear)
      (Variables|Default|SetCurrent%20Distance (Math|Interpolation|FInterptoConstant (Variables|Default|GetCurrent%20Distance) (Variables|Default|GetNext%20Distance) (Variables|Default|GetDelta%20Seconds) 4e+02)))
    (:then_1
      ;[1 0.9184 0.3915] Step 2) Get Location From Spine and update Actor location
      (Utilities|IsValid _track
        (:Is%20Valid
          (Variables|Default|SetTarget%20Location (Spline|GetLocationatDistanceAlongSpline _track (Variables|Default|GetCurrent%20Distance) "World"))
          (Utilities|IsValid _target_point_to_follow
            (:Is%20Valid
              (Transformation|SetActorLocation _target_point_to_follow (Variables|Default|GetTarget%20Location) false false))))))
    (:then_2
      ;[0.5083 1 0.2972] Step 3) Move AI and when Current Distance Nearly Equal Target Spine Point Distance Finish Execute
      (bind _movementresult (AI|AIMoveTo ControlledPawn "0, 0, 0" (Variables|Default|GetTarget%20Point%20to%20Follow) 4e+01 false)
        (:OnSuccess
          (if (Math|Float|NearlyEqual(Float) (Variables|Default|GetCurrent%20Distance) (Variables|Default|GetNext%20Distance) 18.0)
            (Utilities|FlowControl|DoOnce false
              (:Completed
                (Math|Integer|IncrementInt (Variables|Default|GetPointsNumber)
                  (:%20%20
                    (if (== (Variables|Default|GetCurrent%20Point) 1)
                      (Utilities|FlowControl|Delay (Math|Random|RandomFloatinRange 3.0 6.0))
                      (elif (> (Math|Random|RandomFloatinRange 0.0 1.0) 0.8)
                        (Utilities|FlowControl|Delay (Math|Random|RandomFloatinRange 0.6 2.0))))
                    (AI|BehaviorTree|FinishExecute true)))))))
        (:OnFail
          (if (and (Math|Float|NearlyEqual(Float) (Variables|Default|GetCurrent%20Distance) (Variables|Default|GetNext%20Distance) 1.0) (< (Math|Vector|Distance2D(Vector) (Variables|Default|GetTarget%20Location) (Transformation|GetActorLocation ControlledPawn)) 1.6e+02))
            _))))))