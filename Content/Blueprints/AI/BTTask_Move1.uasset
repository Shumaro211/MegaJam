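; Behavior tree task that moves the AI-controlled pawn to a BP_HidePoints actor.
; It loops over all hide points and compares each distance to a threshold that stays at zero, so the last point not at the pawn's location becomes the target.
; After a short delay it runs AIMoveTo, finishing successfully on arrival or repeating the search and move on failure.
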(event EventReceiveExecuteAI
  (params (OwnerController :type AI%20Controller%20Object%20Reference) (ControlledPawn :type Pawn%20Object%20Reference))
  (Variables|Default|Setdistances 0.0)
  (bind _outactors (Actor|GetAllActorsOfClass "/Game/Blueprints/AI/BP_HidePoints.BP_HidePoints_C" :!label _label))
  (for _array_element _outactors
    (if (> (Math|Vector|Distance(Vector) (Transformation|GetActorLocation _array_element) (Transformation|GetActorLocation ControlledPawn)) (Variables|Default|Getdistances))
      (Variables|Default|SetTarget%20Actor _array_element)))
  (Utilities|FlowControl|Delay 0.2)
  (AI|AIMoveTo ControlledPawn "0, 0, 0" (Variables|Default|GetTarget%20Actor) 5.0 false
    (:OnSuccess
      (AI|BehaviorTree|FinishExecute true))
    (:OnFail
      (goto _label))))