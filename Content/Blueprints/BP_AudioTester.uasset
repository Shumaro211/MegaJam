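; BP_AudioTester is an actor that tests audio input by checking whether captured sound reaches a loudness threshold.
; On BeginPlay it starts AudioCapture after a short delay and shows a WB_feedbackTester widget, passing it a self reference.
; Each envelope callback stores the level and maps it against MaxBoo.
; The first full-scale reading, gated by DoOnce, stops capture after a brief delay, prints a pass message and removes the widget.
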(event OnAudioEnvelopeValue(AudioCapture)
  (params (EnvelopeValue :type Float%20%28single-precision%29))
  (bind _output_get (Variables|Default|SetEnvelope%20Value EnvelopeValue))
  (if (== (Math|Float|MapRangeClamped _output_get 0.0 (Variables|Default|GetMaxBoo) 0.0 1.0) 1.0)
    (Utilities|FlowControl|DoOnce false
      (:Completed
        (Utilities|FlowControl|Sequence
          (:then_1
            (Utilities|FlowControl|Delay 0.2)
            (Audio|Components|Audio|Stop (Variables|Default|GetAudioCapture))
            (Development|PrintString "Audio Test Passed!!")
            (Widget|RemovefromParent (Variables|Default|GetSoundTesterWidget))))))))

(event EventBeginPlay
  (Utilities|FlowControl|Delay 0.2)
  (CameraShake|Start (Variables|Default|GetAudioCapture))
  (bind _returnvalue (UserInterface|CreateWidget "/Game/Blueprints/Widgets/WB_feedbackTester.WB_feedbackTester_C" 0 1.0 self))
  (Variables|Default|SetSoundTesterWidget _returnvalue)
  (UserInterface|Viewport|AddtoViewport _returnvalue 0))

(event Collision|EventActorBeginOverlap
  (params (OtherActor :type Actor%20Object%20Reference)))

(event EventTick
  (params (DeltaSeconds :type Float%20%28single-precision%29)))

(fn ConstructionScript)