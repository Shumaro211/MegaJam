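; BP_Mirror is a hauntable mirror interactable that toggles on and off each time Boo fires.
; Switching on plays a shake animation, lights the RectLight, reveals a static mesh and calls AttractHumans.
; Switching off kills the light and hides that mesh.
; Disable clears the on state and light, while CustomDestroy only cuts the light; neither hides the mesh.
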(event EventBeginPlay
  (|CallParentFunction))

(event Collision|EventActorBeginOverlap
  (params (OtherActor :type Actor%20Object%20Reference))
  (|CallParentFunction OtherActor) ; This node is disabled and will not be called.\nDrag off pins to build functionality.
)

(event EventTick
  (params (DeltaSeconds :type Float%20%28single-precision%29))
  (|CallParentFunction DeltaSeconds) ; This node is disabled and will not be called.\nDrag off pins to build functionality.
)

(event EventBoo
  (bind _staticmesh_0 (Variables|Default|GetStaticMesh_0))
  (bind _rectlight (Variables|Default|GetRectLight))
  (|CallParentFunction)
  (if (Variables|Default|GetOn/OFF)
    (Rendering|Components|Light|SetIntensity _rectlight 0.0)
    (Rendering|SetVisibility _staticmesh_0 false false)
    (Variables|Default|SetOn/OFF false)
    (else
      (Components|Animation|PlayAnimation (Variables|Default|GetSkeletalMesh) "/Game/Art/SK/base/shake.shake" false)
      (Rendering|Components|Light|SetIntensity _rectlight 2.4e+04)
      (Rendering|SetVisibility _staticmesh_0 true false)
      (Variables|Default|SetOn/OFF true)
      (CallFunction|AttractHumans))))

(event EventDisable
  (Variables|Default|SetOn/OFF false)
  (Rendering|Components|Light|SetIntensity (Variables|Default|GetRectLight) 0.0))

(event EventCustomDestroy
  (Rendering|Components|Light|SetIntensity (Variables|Default|GetRectLight) 0.0))

(fn ConstructionScript
  (|CallParentFunction))