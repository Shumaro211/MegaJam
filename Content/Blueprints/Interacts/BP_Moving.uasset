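; BP_Moving is an interactable scare prop that, on Boo, attaches to the player and slows their walking.
; While the player moves it, Tick repeatedly triggers a scare in the last overlapped room and attracts humans, throttled by a DoOnce with delayed reset.
; Disable or CustomDestroy detaches it, restores walk speed and lifts the player upward.
; It also registers with its AB_Move anim instance and locks its billboard's yaw.
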(event EventBeginPlay
  (|CallParentFunction)
  (bind _asab_move (Utilities|Casting|CastToAB_Move (Components|SkeletalMesh|GetAnimInstance (Variables|Default|GetSkeletalMesh))))
  (Variables|/Game/Art/SK/AB_Move.AB_Move_C|SetOwnerActor _asab_move self))

(event Collision|EventActorBeginOverlap
  (params (OtherActor :type Actor%20Object%20Reference))
  (bind _asbp_room (Utilities|Casting|CastToBP_Room OtherActor))
  (Variables|Default|SetRoom _asbp_room))

(event EventTick
  (params (DeltaSeconds :type Float%20%28single-precision%29))
  (bind _billboard (Variables|Default|GetBillboard))
  (bind _returnvalue (Transformation|GetWorldRotation _billboard))
  (|CallParentFunction DeltaSeconds)
  (Transformation|SetWorldRotation _billboard (Math|Rotator|MakeRotator (.roll _returnvalue) (.pitch _returnvalue) -9e+01) false false)
  (if (Variables|Default|GetBooDone)
    (if (> (Math|Vector|VectorLength (Transformation|GetVelocity (Game|Player|GetPlayerPawn 0))) 1e+01)
      (Utilities|FlowControl|DoOnce false :!label _label
        (:Completed
          (Utilities|FlowControl|Sequence
            (:then_0
              (Default|Trigger (Variables|Default|GetRoom) (Variables|Default|GetScareFactor) self)
              (CallFunction|AttractHumans))
            (:then_1
              (Utilities|FlowControl|Delay 1.4)
              (goto _label Reset))))))))

(event EventBoo
  (bind _returnvalue (Game|Player|GetPlayerPawn 0))
  (bind _returnvalue_2 (Transformation|GetActorLocation _returnvalue))
  (|CallParentFunction)
  (CallFunction|AttractHumans)
  (Transformation|SetActorLocation (Math|Vector|MakeVector (.x _returnvalue_2) (.y _returnvalue_2) (.z (Transformation|GetActorLocation))) false false)
  (Transformation|AttachActorToActor (Game|Player|GetPlayerPawn 0) "None" "KeepWorld" "KeepWorld" "KeepRelative" true)
  (Variables|Default|SetBooDone true)
  (bind _asbp_top_down_character (Utilities|Casting|CastToBP_TopDownCharacter (Game|Player|GetPlayerPawn 0)))
  (Variables|/Script/Engine.CharacterMovementComponent|SetMaxWalkSpeed (Variables|/Script/Engine.Character|GetCharacterMovement _asbp_top_down_character) 2.4e+02))

(event EventDisable
  (Variables|Default|SetBooDone false)
  (Transformation|DetachFromActor "KeepWorld" "KeepWorld" "KeepRelative")
  (bind _asbp_top_down_character (Utilities|Casting|CastToBP_TopDownCharacter (Game|Player|GetPlayerPawn 0)))
  (Variables|/Script/Engine.CharacterMovementComponent|SetMaxWalkSpeed (Variables|/Script/Engine.Character|GetCharacterMovement _asbp_top_down_character) 5.7e+02)
  (Transformation|SetActorLocation _asbp_top_down_character (+ (Transformation|GetActorLocation _asbp_top_down_character) "0.000000,0.000000,80.000000") false false))

(event EventCustomDestroy
  (Variables|Default|SetBooDone false)
  (Transformation|DetachFromActor "KeepWorld" "KeepWorld" "KeepRelative")
  (bind _asbp_top_down_character (Utilities|Casting|CastToBP_TopDownCharacter (Game|Player|GetPlayerPawn 0)))
  (Variables|/Script/Engine.CharacterMovementComponent|SetMaxWalkSpeed (Variables|/Script/Engine.Character|GetCharacterMovement _asbp_top_down_character) 5.7e+02)
  (Transformation|SetActorLocation _asbp_top_down_character (+ (Transformation|GetActorLocation _asbp_top_down_character) "0.000000,0.000000,80.000000") false false))

(fn ConstructionScript
  (|CallParentFunction))