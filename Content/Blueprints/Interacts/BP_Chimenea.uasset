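; BP_Chimenea is an interactable fireplace that lights up and attracts humans when its Boo event fires.
; Boo runs the parent logic, then makes the fire mesh and point light visible.
; A timeline lerps the mesh's world scale and the light's intensity to grow the flame.
; The same event then calls AttractHumans right after starting the timeline, without waiting for it to finish.
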(event EventBeginPlay
  (|CallParentFunction))

(event Collision|EventActorBeginOverlap
  (params (OtherActor :type Actor%20Object%20Reference))
  (|CallParentFunction OtherActor) ; This node is disabled and will not be called.\nDrag off pins to build functionality.
)

(event EventTick
  (params (DeltaSeconds :type Float%20%28single-precision%29))
  (|CallParentFunction DeltaSeconds) ; This node is disabled and will not be called.\nDrag off pins to build functionality.
)

(event EventBoo
  (|CallParentFunction)
  (Utilities|FlowControl|Sequence
    (:then_0
      (Rendering|SetVisibility (Variables|Default|GetSM_Fire) true false)
      (Rendering|SetVisibility (Variables|Default|GetPointLight) true false)
      (bind _newtrack_0 (Timeline|Timeline_0 Play)
        (:Update
          (Transformation|SetWorldScale3D (Variables|Default|GetSM_Fire) (Math|Vector|Lerp(Vector) "0.100000,0.100000,0.100000" "0.350000,0.350000,0.350000" _newtrack_0))
          (Rendering|Components|Light|SetIntensity (Variables|Default|GetPointLight) (Math|Float|Lerp 5e+02 3e+03 _newtrack_0)))))
    (:then_1
      (CallFunction|AttractHumans))))

(fn ConstructionScript
  (|CallParentFunction))