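; Window interactable that responds to the Boo event by sliding open or shut and drawing humans' attention.
; Each Boo runs the parent behavior, then a FlipFlop alternately plays and reverses the CloseOpen timeline.
; The timeline lerps the Sphere component's relative Y position between two fixed offsets, and AttractHumans fires when it finishes.
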(event EventBeginPlay
  (|CallParentFunction) ; This node is disabled and will not be called.\nDrag off pins to build functionality.
)

(event Collision|EventActorBeginOverlap
  (params (OtherActor :type Actor%20Object%20Reference)))

(event EventTick
  (params (DeltaSeconds :type Float%20%28single-precision%29))
  (|CallParentFunction DeltaSeconds) ; This node is disabled and will not be called.\nDrag off pins to build functionality.
)

(event EventBoo
  (bind _sphere (Variables|Default|GetSphere))
  (bind _relativelocation (Variables|/Script/Engine.SceneComponent|GetRelativeLocation _sphere))
  (|CallParentFunction)
  (Utilities|FlowControl|Sequence
    (:then_0
      (Utilities|FlowControl|FlipFlop
        (:A
          (bind _move (Timeline|CloseOpen Play)
            (:Update
              (Transformation|SetRelativeLocation _sphere (Math|Vector|MakeVector (.x _relativelocation) (Math|Float|Lerp -1.7e+02 -8e+01 _move) (.z _relativelocation)) false false))
            (:Finished
              (CallFunction|AttractHumans))))
        (:B
          (Timeline|CloseOpen Reverse))))))

(fn ConstructionScript
  (|CallParentFunction))