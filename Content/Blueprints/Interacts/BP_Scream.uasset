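; BP_Scream is an interactable scare that plays a ghost lady scream and frightens every human in the level.
; CustomInt raises Sensibility after a short delay, cuts the custom camera to BP_Camera and hands itself to the ghost's animation instance.
; Boo waits, changes the target human's AI state, attracts and scares all humans, and returns the camera to the player.
; Tick holds the billboard at a fixed yaw.
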(event EventTick
  (params (DeltaSeconds :type Float%20%28single-precision%29))
  (bind _billboard (Variables|Default|GetBillboard))
  (bind _returnvalue (Transformation|GetWorldRotation _billboard))
  (Transformation|SetWorldRotation _billboard (Math|Rotator|MakeRotator (.roll _returnvalue) (.pitch _returnvalue) -9e+01) false false))

(event EventBoo
  (|CallParentFunction)
  (bind _asbp_human (Utilities|Casting|CastToBP_Human (Variables|Default|GetTarget)))
  (Utilities|FlowControl|Delay 3.5)
  (Utilities|FlowControl|Sequence
    (:then_0
      (Default|ChangeState (Variables|/Game/ThirdPerson/Blueprints/BP_Human.BP_Human_C|GetNPCAI _asbp_human) "NewEnumerator8")
      (Utilities|FlowControl|Delay 0.2)
      (CallFunction|AttractHumans)
      (bind _outactors (Actor|GetAllActorsOfClass "/Game/ThirdPerson/Blueprints/BP_Human.BP_Human_C"))
      (for _array_element _outactors
        (Default|Scare _array_element 50 self)))
    (:then_1
      (bind _ascustom_camera (Utilities|Casting|CastToCustomCamera (Variables|/Script/Engine.PlayerController|GetPlayerCameraManager (Game|GetPlayerController 0))))
      (bind _asbp_top_down_character (Utilities|Casting|CastToBP_TopDownCharacter (Game|Player|GetPlayerPawn 0)))
      (Variables|/Game/Blueprints/CustomCamera.CustomCamera_C|SetCamera _ascustom_camera (Variables|/Game/TopDown/Blueprints/BP_TopDownCharacter.BP_TopDownCharacter_C|GetCamera _asbp_top_down_character))
      (Variables|/Game/Blueprints/CustomCamera.CustomCamera_C|SetPlayer? _ascustom_camera true))))

(event EventCustomInt
  (Utilities|FlowControl|Delay 0.4)
  (Variables|Default|SetSensibility (+ (Variables|Default|GetSensibility) (* (/ (Variables|Default|GetSensibility) 1e+01) 1.7)))
  (bind _returnvalue (Actor|GetActorOfClass "/Game/Blueprints/BP_Camera.BP_Camera_C"))
  (bind _ascustom_camera (Utilities|Casting|CastToCustomCamera (Variables|/Script/Engine.PlayerController|GetPlayerCameraManager (Game|GetPlayerController 0))))
  (Variables|/Game/Blueprints/CustomCamera.CustomCamera_C|SetCamera _ascustom_camera (Variables|/Game/Blueprints/BP_Camera.BP_Camera_C|GetCamera _returnvalue))
  (Variables|/Game/Blueprints/CustomCamera.CustomCamera_C|SetPlayer? _ascustom_camera false)
  (bind _returnvalue_2 (Actor|GetActorOfClass "/Game/Blueprints/BP_GhostAnim.BP_GhostAnim_C"))
  (bind _asghost_lady_scream (Utilities|Casting|CastToGhostLady_Scream (Components|SkeletalMesh|GetAnimInstance (Variables|/Game/Blueprints/BP_GhostAnim.BP_GhostAnim_C|GetSkeletalMesh _returnvalue_2))))
  (Variables|/Game/Art/Characters/GhostLadyAnim/GhostLady_Scream.GhostLady_Scream_C|Setscream _asghost_lady_scream -1.0)
  (Default|SetGhsot _asghost_lady_scream self))

(fn ConstructionScript
  (|CallParentFunction))