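; BP_Fall is an interactable object that falls when booed and attracts humans.
; It overrides Boo, calling the parent logic, then playing the Fall1 animation once on its skeletal mesh.
; A short fixed delay follows before it calls AttractHumans.
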(event EventBeginPlay
  (|CallParentFunction) ; This node is disabled and will not be called.\nDrag off pins to build functionality.
)

(event Collision|EventActorBeginOverlap
  (params (OtherActor :type Actor%20Object%20Reference)))

(event EventTick
  (params (DeltaSeconds :type Float%20%28single-precision%29))
  (|CallParentFunction DeltaSeconds) ; This node is disabled and will not be called.\nDrag off pins to build functionality.
)

(event EventBoo
  (|CallParentFunction)
  (Components|Animation|PlayAnimation (Variables|Default|GetSkeletalMesh) "/Game/Art/SK/base/fall1.fall1" false)
  (Utilities|FlowControl|Delay 0.82)
  (CallFunction|AttractHumans))

(fn ConstructionScript
  (|CallParentFunction))