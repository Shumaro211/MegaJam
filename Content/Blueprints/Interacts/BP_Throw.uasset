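; BP_Throw is a scare interactable that throws a spawned actor when booed, then attracts humans.
; Boo runs the parent logic, plays the Book animation, and after a short delay spawns the configured Class at the Fire component's transform.
; It then increments Amount and, after another delay, calls AttractHumans.
; The MaxAmount check is disconnected, so this graph does not cap throws.
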(event EventBeginPlay
  (|CallParentFunction) ; This node is disabled and will not be called.\nDrag off pins to build functionality.
)

(event Collision|EventActorBeginOverlap
  (params (OtherActor :type Actor%20Object%20Reference)))

(event EventTick
  (params (DeltaSeconds :type Float%20%28single-precision%29))
  (|CallParentFunction DeltaSeconds) ; This node is disabled and will not be called.\nDrag off pins to build functionality.
)

(event EventBoo
  (|CallParentFunction)
  (Components|Animation|PlayAnimation (Variables|Default|GetSkeletalMesh) "/Game/Art/SK/base/book.book" false)
  (Utilities|FlowControl|Delay 0.2)
  (Game|SpawnActorfromClass (Variables|Default|GetClass) (Transformation|GetWorldTransform (Variables|Default|Getfire)) "AdjustIfPossibleButAlwaysSpawn" "MultiplyWithRoot" 0 0)
  (Math|Integer|IncrementInt (Variables|Default|GetAmount)
    (:%20%20
      (Utilities|FlowControl|Delay 0.5)
      (CallFunction|AttractHumans))))

(fn ConstructionScript
  (|CallParentFunction))