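; BP_Room is a room volume that relays scares to the humans inside and tracks whether its light is on.
; Trigger scares overlapping BP_Humans, halving the incoming strength while lit before adding a flat bonus, with a short re-trigger lockout.
; It also arms a one-off SmallScare for the next human to enter; entry sets their CurrentRoom.
; IsSeeingGhost checks whether a given human shares the box with BP_TopDownCharacter.
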(event OnComponentBeginOverlap(Box)
  (params (OverlappedComponent :type Primitive%20Component%20Object%20Reference) (OtherActor :type Actor%20Object%20Reference) (OtherComp :type Primitive%20Component%20Object%20Reference) (OtherBodyIndex :type Integer) (bFromSweep :type Boolean) (SweepResult :type Hit%20Result%20Structure%20%28by%20ref%29))
  (bind _asbp_human (Utilities|Casting|CastToBP_Human OtherActor))
  (Variables|/Game/ThirdPerson/Blueprints/BP_Human.BP_Human_C|SetCurrentRoom _asbp_human self)
  (if (Variables|Default|GetActiveObject)
    (Variables|Default|SetActiveObject false)
    (Default|SmallScare _asbp_human)))

(event OnComponentEndOverlap(Box)
  (params (OverlappedComponent :type Primitive%20Component%20Object%20Reference) (OtherActor :type Actor%20Object%20Reference) (OtherComp :type Primitive%20Component%20Object%20Reference) (OtherBodyIndex :type Integer)))

(event Custom|Trigger
  (params (B :type Integer) (Source :type Actor%20Object%20Reference))
  (Utilities|FlowControl|Sequence
    (:then_0
      (Utilities|FlowControl|DoOnce false :!label _label
        (:Completed
          (Utilities|FlowControl|Sequence
            (:then_0
              (for _array_element (Collision|GetOverlappingActors (Variables|Default|GetBox) "/Game/ThirdPerson/Blueprints/BP_Human.BP_Human_C" :!class /Script/Engine.PrimitiveComponent)
                (bind _asbp_human (Utilities|Casting|CastToBP_Human _array_element))
                (Default|Scare _asbp_human (+ (/ B (Math|Integer|SelectInt 2 1 (Variables|Default|GetLight?))) 4) Source)
                (Development|PrintString (Utilities|GetDisplayName Source))))
            (:then_1
              (Utilities|FlowControl|Delay 0.2)
              (goto _label Reset))))))
    (:then_1
      (Variables|Default|SetActiveObject true))))

(event Custom|NoLight
  (Variables|Default|SetLight? false))

(event EventBeginPlay
  (bind _light (Variables|Default|GetLight))
  (bind _light_table (Variables|Default|GetLight_Table))
  (Utilities|IsValid _light
    (:Is%20Valid
      (Variables|Default|SetLight? true)
      (EventDispatchers|BindEventtoDestroyedLight _light (delegate Custom|NoLight)))
    (:Is%20Not%20Valid
      (Utilities|IsValid _light_table
        (:Is%20Valid
          (Variables|Default|SetLight? true)
          (EventDispatchers|BindEventtoDestroyedLight _light_table (delegate Custom|NoLight)))))))

(fn ConstructionScript)

(fn IsSeeingGhost
  (params (ItemToFind :type Actor%20Object%20Reference%20%28by%20ref%29))
  (if (Utilities|Array|ContainsItem (Collision|GetOverlappingActors (Variables|Default|GetBox) "/Game/ThirdPerson/Blueprints/BP_Human.BP_Human_C" :!class /Script/Engine.PrimitiveComponent) ItemToFind)
    (Utilities|IsValid (Utilities|Array|Get(acopy) (Collision|GetOverlappingActors (Variables|Default|GetBox) "/Game/TopDown/Blueprints/BP_TopDownCharacter.BP_TopDownCharacter_C" :!class /Script/Engine.PrimitiveComponent))
      (:Is%20Valid
        (return)))))