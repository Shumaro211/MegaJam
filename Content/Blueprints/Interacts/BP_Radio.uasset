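; Radio interactable that a Boo event toggles on and off, luring humans while it plays.
; Switching on starts audio, a shake animation and a visible static mesh, then opens a Gate that loops AttractHumans every 1.1 seconds until closed or destroyed.
; Disable and CustomDestroy share one shutdown path that silences audio, hides the mesh and closes the Gate.
; A timeline-driven mesh scaling effect is present but never runs.
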(event EventBeginPlay
  (|CallParentFunction)
  (Components|Timeline|SetPlayRate (Variables|Default|GetTimeline_0) 0.2))

(event Collision|EventActorBeginOverlap
  (params (OtherActor :type Actor%20Object%20Reference))
  (|CallParentFunction OtherActor) ; This node is disabled and will not be called.\nDrag off pins to build functionality.
)

(event EventTick
  (params (DeltaSeconds :type Float%20%28single-precision%29))
  (|CallParentFunction DeltaSeconds) ; This node is disabled and will not be called.\nDrag off pins to build functionality.
)

(event EventBoo
  (bind _staticmesh_0 (Variables|Default|GetStaticMesh_0))
  (bind _audio (Variables|Default|GetAudio))
  (|CallParentFunction)
  (if (Variables|Default|GetOn/OFF)
    (Audio|Components|Audio|Stop _audio)
    (Rendering|SetVisibility _staticmesh_0 false false)
    (Variables|Default|SetOn/OFF false)
    (goto _label Close)
    (else
      (Audio|Components|Audio|Play _audio 0.0)
      (Components|Animation|PlayAnimation (Variables|Default|GetSkeletalMesh) "/Game/Art/SK/base/shake.shake" false)
      (Rendering|SetVisibility _staticmesh_0 true false)
      (Variables|Default|SetOn/OFF true)
      (Utilities|FlowControl|Sequence
        (:then_0
          (goto _label Open))
        (:then_1
          (Utilities|FlowControl|Gate false :!label _label
            (:Exit
              (CallFunction|AttractHumans)
              (Utilities|FlowControl|Delay 1.1)
              (if (Variables|Default|GetDestroyed?)
                (Audio|Components|Audio|Stop (Variables|Default|GetAudio))
                (else
                  (goto _label))))))))))

(event EventDisable
  (Audio|Components|Audio|Stop (Variables|Default|GetAudio))
  (Variables|Default|SetOn/OFF false)
  (Audio|Components|Audio|Stop (Variables|Default|GetTimeline_0))
  (Rendering|SetVisibility (Variables|Default|GetStaticMesh_0) false false)
  (Utilities|FlowControl|Gate false) ; enters at Close
)

(event EventCustomDestroy
  (Audio|Components|Audio|Stop (Variables|Default|GetAudio))
  (Variables|Default|SetOn/OFF false)
  (Audio|Components|Audio|Stop (Variables|Default|GetTimeline_0))
  (Rendering|SetVisibility (Variables|Default|GetStaticMesh_0) false false)
  (Utilities|FlowControl|Gate false) ; enters at Close
)

(fn ConstructionScript
  (|CallParentFunction))